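; Enemy attack component that applies melee trace damage from its owner.
; StartAttackTrace stores the damage and schedules AttackTrace on a short timer, which StopAttackTrace clears.
; The trace sphere-casts on Visibility from the owner's second Arrow component to an offset in its local space, with persistent debug drawing, and applies the stored damage to the hit actor.
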(event `StartAttackTrace`
  (params (Damage :type "Float (double-precision)"))
  (set `self.CurrentActorDamage` Damage)
  (bind _returnvalue (`KismetSystemLibrary.K2_SetTimerDelegate` (delegate `AttackTrace`) 0.01))
  (set `self.Attack Timer Handler` _returnvalue))

(event `AttackTrace`
  (bind _output (`|GetArrayItem` (`Actor.K2_GetComponentsByClass` (`self.GetOwner`) "/Script/Engine.ArrowComponent") 1))
  (`|ExecutionSequence`
    (:`then_1`
      (bind _outhit (`KismetSystemLibrary.SphereTraceSingle` :`Start` (`SceneComponent.K2_GetComponentLocation` _output) :`End` (`KismetMathLibrary.TransformLocation` (`SceneComponent.K2_GetComponentToWorld` _output) (+ (`SceneComponent.RelativeLocation` _output) (20.0 0.0 0.0))) :`Radius` (`self.CollisionRadius`) :`TraceChannel` "TraceTypeQuery1" :`DrawDebugType` "Persistent"))
      (`GameplayStatics.ApplyDamage` (`.HitActor` (`GameplayStatics.BreakHitResult` _outhit)) (`self.CurrentActorDamage`) null (`self.GetOwner`)))))

(event `StopAttackTrace`
  (`KismetSystemLibrary.K2_ClearAndInvalidateTimerHandle` (`self.Attack Timer Handler`)))