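; Player attack component that runs timed melee hit traces and applies damage.
; StartAttackTrace stores damage and starts a fast looping timer until StopAttackTrace; each tick sphere-traces the owner's first attached item and damages the hit actor, with persistent debug drawing.
; The trace uses hardcoded socket names, ignoring the stored socket inputs, and does not filter repeat hits.
; ResetByHit clears the attacking flag when the player is stunned.
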(event `StartAttackTrace`
  (params (Damage :type "Float (double-precision)") (InStartSocket :type Name) (InEndSocket :type Name))
  (set `self.In Start Socket` InStartSocket)
  (set `self.In End Socket` InEndSocket)
  (set `self.CurrentActorDamage` Damage)
  (bind _returnvalue (`KismetSystemLibrary.K2_SetTimerDelegate` (delegate `AttackTrace`) 0.01 true))
  (set `self.Attack Timer Handler` _returnvalue))

(event `AttackTrace`
  (`|ExecutionSequence`
    (:`then_1`
      (bind _asbp_item_base (cast `/Game/UtubeInventory/Items/BP_Item_Base` (`|GetArrayItem` (`Actor.GetAttachedActors` (`self.GetOwner`) true false))))
      (bind _itemmesh (`/Game/UtubeInventory/Items/BP_Item_Base.ItemMesh` _asbp_item_base))
      (bind _outhit (`KismetSystemLibrary.SphereTraceSingle` :`Start` (`SceneComponent.GetSocketLocation` _itemmesh "Hand1Tip") :`End` (`SceneComponent.GetSocketLocation` _itemmesh "Weapon1Tip") :`Radius` 30.0 :`TraceChannel` "TraceTypeQuery1" :`DrawDebugType` "Persistent"))
      (`GameplayStatics.ApplyDamage` (`.HitActor` (`GameplayStatics.BreakHitResult` _outhit)) (`self.CurrentActorDamage`)))))

(event `StopAttackTrace`
  (`KismetSystemLibrary.K2_ClearAndInvalidateTimerHandle` (`self.Attack Timer Handler`)))

(event `ResetByHit`
  (if (`/Game/ThirdPerson/Blueprints/BP_FightThirdPerson/BP_FightThirdPerson.IsStunned` (`self.PlayerCharacter`))
    (set `self.IsAttacking` false)))

(event `self.ReceiveBeginPlay`)