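; Health component that applies damage to its owning actor and destroys that actor when health runs out.
; TakeDamge skips if IsDead, otherwise subtracts damage, clamps CurrentHealth between zero and MaxHealth, and broadcasts OnHealthChanged.
; At zero health it destroys the owner, then finds DoorManager actors and calls Check on them.
; The event graph holds no logic, and IsDead is only read here, never set.
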(fn `TakeDamge`
  (params (DamageAmount :type "Float (double-precision)"))
  (if (not (`self.IsDead`))
    (bind _output_get (set `self.CurrentHealth` (`KismetMathLibrary.FClamp` (- (`self.CurrentHealth`) DamageAmount) 0.0 (`self.MaxHealth`))))
    (`self.OnHealthChanged` _output_get (`self.MaxHealth`))
    (if (<= (`self.CurrentHealth`) 0.0)
      (`Actor.K2_DestroyActor` (`self.GetOwner`))
      (bind _outactors (`GameplayStatics.GetAllActorsOfClass` "/Game/Tool/DoorManager.DoorManager_C"))
      (`/Game/Tool/DoorManager.Check` _outactors))))