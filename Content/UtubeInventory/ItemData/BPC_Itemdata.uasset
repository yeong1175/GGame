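; Actor component that makes its owning actor a pickup item for the inventory system, holding a data table row handle and a quantity.
; Interacting passes the row name and quantity to the interactor's BPC_EasyInventory component and destroys the owner if pickup succeeds.
; GetItemData looks up the row from the stored handle, ignoring its ItemID input, and Lookat returns an empty string.
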(event `/Game/UtubeInventory/Interaction/Interaction/Bpi_Interaction.InteractWith`
  (params (Interactor :type "Actor Object Reference"))
  (`self.PickUp` Interactor))

(event `PickUp`
  (params (interactactor :type "Actor Object Reference"))
  (bind _returnvalue (`Actor.GetComponentByClass` interactactor "/Game/UtubeInventory/Inventory/BPC_EasyInventory.BPC_EasyInventory_C"))
  (`/Engine/EditorBlueprintResources/StandardMacros.IsValid` _returnvalue
    (:`Is Valid`
      (bind _success (`/Game/UtubeInventory/Inventory/BPC_EasyInventory.PickUp` _returnvalue (`.RowName` (break `DataTableRowHandle` (`self.ItemData`))) (`self.ItemQuantity`)))
      (if _success
        (`Actor.K2_DestroyActor` (`self.GetOwner`))))))

(fn `GetItemData`
  (params (ItemID :type Name))
  (returns (ItemData :type "/Game/UtubeInventory/ItemData/S_ItemInfo Structure"))
  (bind (_datatable _rowname) (break `DataTableRowHandle` (`self.ItemData`)))
  (bind _returnvalue (`|GetDataTableRow` _datatable _rowname)
    (:`then`
      (return _returnvalue))))

(fn `Lookat`
  (returns (Message :type Text))
  (return ""))