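; Slot-based inventory component that handles picking up, stacking, transferring, dropping and equipping items.
; ItemSlots hold ID and quantity, while DT_ItemData supplies stack limits and actor classes; changes broadcast OnInventoryUpdated.
; Pickup fills a matching stack or empty slot, and transfers merge matching items with overflow or swap different ones.
; Drops spawn in a cone ahead of the owner; equipping attaches a spawned actor to BP_FightThirdPerson's right-hand socket.
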(event `self.ReceiveBeginPlay`
  (`KismetArrayLibrary.Array_Resize` (`self.ItemSlots`) (`self.InventorySize`)))

(event `UpdateInventory`
  (`self.OnInventoryUpdated`))

(fn `AddtoNewSlot`
  (params (ItemID :type Name) (ItemQuantity :type Integer) (Index :type Integer))
  (`KismetArrayLibrary.Array_Set` (`self.ItemSlots`) Index (make `/Game/UtubeInventory/ItemData/S_ItemSlot` ItemID ItemQuantity)))

(fn `AddtoSlot`
  (params (Index :type Integer) (ItemQuantity :type Integer))
  (bind (_output_itemid _output_itemquantity) (break `/Game/UtubeInventory/ItemData/S_ItemSlot` (`|GetArrayItem` (`self.ItemSlots`) Index)))
  (`KismetArrayLibrary.Array_Set` (`self.ItemSlots`) (`local.Index`) (make `/Game/UtubeInventory/ItemData/S_ItemSlot` _output_itemid (+ _output_itemquantity (`local.ItemQuantity`)))))

(fn `AnyAvalableSlots`
  (returns (Success :type Boolean) (Index :type Integer))
  (for (_array_element _array_index) (`self.ItemSlots`)
    (if (== (`.ItemQuantity_6_A626BBD4463E6CB7B64186916546EB7E` (break `/Game/UtubeInventory/ItemData/S_ItemSlot` _array_element)) 0)
      (return true _array_index)))
  (return false -1))

(fn `DropFromInventory`
  (params (ItemID :type Name) (ItemQuantity :type Integer) (Index :type Integer))
  (for _ (range ItemQuantity)
    (`|SpawnActorFromClass` (`.Item_Class_17_C6C868DA42EC70B6210F64830FA20DC9` (break `/Game/UtubeInventory/ItemData/S_ItemInfo` (`self.GetItemData` (`local.ItemID`)))) (`KismetMathLibrary.MakeTransform` (`self.GetDropLocation`)) "Undefined" "MultiplyWithRoot" null null)
    (`KismetArrayLibrary.Array_Set` (`self.ItemSlots`) (`local.Index`) (make `/Game/UtubeInventory/ItemData/S_ItemSlot` "None"))
    (`self.UpdateInventory`)))

(fn `EquipItem`
  (params (SlotIndex :type Integer) (ItemID :type Name))
  (bind _currentequippedactor (`self.CurrentEquippedActor`))
  (bind (_item_name _item_icon _item_class) (break `/Game/UtubeInventory/ItemData/S_ItemInfo` (`self.GetItemData` ItemID)))
  (if (`KismetSystemLibrary.IsValidClass` _item_class)
    (`KismetSystemLibrary.PrintString` (`KismetSystemLibrary.GetClassDisplayName` _item_class))
    (`/Engine/EditorBlueprintResources/StandardMacros.IsValid` _currentequippedactor
      (:`Is Valid`
        (`Actor.K2_DestroyActor` _currentequippedactor))
      (:`Is Not Valid`
        _))
    (bind _returnvalue (`|SpawnActorFromClass` _item_class (`KismetMathLibrary.MakeTransform` (0.0 0.0 0.0)) "AlwaysSpawn" "MultiplyWithRoot" null null))
    (bind _output_get (set `self.CurrentEquippedActor` _returnvalue))
    (`Actor.SetActorEnableCollision` _output_get false)
    (bind _itemmesh (`/Game/UtubeInventory/Items/BP_Item_Base.ItemMesh` _returnvalue))
    (`PrimitiveComponent.SetSimulatePhysics` _itemmesh false)
    (bind _asbp_fight_third_person (cast `/Game/ThirdPerson/Blueprints/BP_FightThirdPerson/BP_FightThirdPerson` (`self.GetOwner`)))
    (`SceneComponent.K2_AttachToComponent` _itemmesh (`Character.Mesh` _asbp_fight_third_person) "Hand_R_Socket" "KeepRelative" "KeepRelative" "KeepRelative" true)
    (`KismetArrayLibrary.Array_Set` (`self.ItemSlots`) SlotIndex (make `/Game/UtubeInventory/ItemData/S_ItemSlot` "None"))
    (`self.UpdateInventory`)))

(fn `FindMatchingSlot`
  (params (ItemID :type Name))
  (returns (Success :type Boolean) (Index :type Integer))
  (for (_array_element _array_index) (`self.ItemSlots`)
    (bind (_itemid _itemquantity) (break `/Game/UtubeInventory/ItemData/S_ItemSlot` _array_element))
    (if (and (== (`local.ItemID`) _itemid) (< _itemquantity (`.Item_Quantity_14_35E8F06A4E69E098735BCBB82C9930E6` (break `/Game/UtubeInventory/ItemData/S_ItemInfo` (`self.GetItemData` (`local.ItemID`))))))
      (return true _array_index)))
  (return false -1))

(fn `GetDropLocation`
  (returns (DropLocation :type "Vector Structure"))
  (bind _returnvalue (`self.GetOwner`))
  (return (+ (`Actor.K2_GetActorLocation` _returnvalue) (* (`KismetMathLibrary.RandomUnitVectorInConeInDegrees` (`Actor.GetActorForwardVector` _returnvalue) 55.0) 100.0))))

(fn `GetItemData`
  (params (ItemID :type Name))
  (returns (ItemData :type "/Game/UtubeInventory/ItemData/S_ItemInfo Structure"))
  (bind _returnvalue (`|GetDataTableRow` "/Game/UtubeInventory/ItemData/DT_ItemData.DT_ItemData" ItemID)
    (:`then`
      (return _returnvalue))))

(fn `ItemTransfer`
  (params (SourceInventory :type "/Game/UtubeInventory/Inventory/BPC_EasyInventory Object Reference") (SourceSlot :type "/Game/UtubeInventory/ItemData/S_ItemSlot Structure") (DestinationSlot :type "/Game/UtubeInventory/ItemData/S_ItemSlot Structure") (Index :type Integer) (SourceIndex :type Integer))
  (locals (LocalTotalSum :type Integer) (Local_SubtratedSum :type Integer))
  (bind (_itemid _itemquantity) (break `/Game/UtubeInventory/ItemData/S_ItemSlot` (`local.SourceSlot`)))
  (bind (_item_name _item_icon _item_class _item_sfx _item_quantity) (break `/Game/UtubeInventory/ItemData/S_ItemInfo` (`self.GetItemData` (`.ItemID_4_D9725D3941C812239EFE3E94C6925D23` (break `/Game/UtubeInventory/ItemData/S_ItemSlot` (`local.SourceSlot`))))))
  (bind _output_get (set `local.LocalTotalSum` (+ _itemquantity (`.ItemQuantity_6_A626BBD4463E6CB7B64186916546EB7E` (break `/Game/UtubeInventory/ItemData/S_ItemSlot` (`local.DestinationSlot`))))))
  (if (> _output_get (`.Item_Quantity_14_35E8F06A4E69E098735BCBB82C9930E6` (break `/Game/UtubeInventory/ItemData/S_ItemInfo` (`self.GetItemData` _itemid))))
    (set `local.Local_SubtratedSum` (- (`local.LocalTotalSum`) _item_quantity))
    (`self.AddtoNewSlot` (`.ItemID_4_D9725D3941C812239EFE3E94C6925D23` (break `/Game/UtubeInventory/ItemData/S_ItemSlot` (`local.SourceSlot`))) _item_quantity (`local.Index`))
    (`self.AddtoNewSlot` (`local.SourceInventory`) (`.ItemID_4_D9725D3941C812239EFE3E94C6925D23` (break `/Game/UtubeInventory/ItemData/S_ItemSlot` (`local.SourceSlot`))) (`local.Local_SubtratedSum`) (`local.SourceIndex`))
    (else
      (`self.AddtoNewSlot` (`.ItemID_4_D9725D3941C812239EFE3E94C6925D23` (break `/Game/UtubeInventory/ItemData/S_ItemSlot` (`local.SourceSlot`))) (`local.LocalTotalSum`) (`local.Index`))
      (`self.AddtoNewSlot` (`local.SourceInventory`) "None" 0 (`local.SourceIndex`)))))

(fn `PickUp`
  (params (ItemID :type Name) (ItemQuantity :type Integer))
  (returns (Success :type Boolean) (ItemQuantityLeft :type Integer))
  (locals (LocalItemQuantity :type Integer) (Local_IsFull :type Boolean :default false))
  (bind (_success _index) (`self.AnyAvalableSlots`))
  (bind _output_get (set `local.LocalItemQuantity` ItemQuantity))
  (while (and (> _output_get 0) (not (`local.Local_IsFull`)))
    (bind (_success_2 _index_2) (`self.FindMatchingSlot` (`local.ItemID`)))
    (if _success_2
      (`self.AddtoSlot` _index_2 1)
      (`/Engine/EditorBlueprintResources/StandardMacros.DecrementInt` (`local.LocalItemQuantity`) :!label _label
        (:`  `
          (`self.UpdateInventory`)
          (return true 0)))
      (elif _success
        (`self.AddtoNewSlot` (`local.ItemID`) 1 _index)
        (goto _label))))
  (`self.UpdateInventory`)
  (return (not (`local.Local_IsFull`)) (`local.LocalItemQuantity`)))

(fn `PrintInventory`
  (for (_array_element _array_index) (`self.ItemSlots`)
    (bind (_itemid _itemquantity) (break `/Game/UtubeInventory/ItemData/S_ItemSlot` _array_element))
    (`KismetSystemLibrary.PrintString` (`KismetStringLibrary.Concat_StrStr` (`KismetStringLibrary.Conv_IntToString` _array_index) " :" (`KismetStringLibrary.Conv_NameToString` _itemid) " =" (`KismetStringLibrary.Conv_IntToString` _itemquantity)))))

(fn `TransferSlots`
  (params (Index :type Integer) (SourceIndex :type Integer) (SourceInventory :type "/Game/UtubeInventory/Inventory/BPC_EasyInventory Object Reference"))
  (locals (LocalDestinationInventory :type "/Game/UtubeInventory/ItemData/S_ItemSlot Structure") (LocalSourceInventory :type "/Game/UtubeInventory/ItemData/S_ItemSlot Structure"))
  (bind (_itemid _itemquantity) (break `/Game/UtubeInventory/ItemData/S_ItemSlot` (`local.LocalDestinationInventory`)))
  (bind (_itemid_2 _itemquantity_2) (break `/Game/UtubeInventory/ItemData/S_ItemSlot` (`local.LocalSourceInventory`)))
  (set `local.LocalDestinationInventory` (`|GetArrayItem` (`self.ItemSlots`) (`local.Index`)))
  (set `local.LocalSourceInventory` (`|GetArrayItem` (`/Game/UtubeInventory/Inventory/BPC_EasyInventory.ItemSlots` (`local.SourceInventory`)) (`local.SourceIndex`)))
  (`|ExecutionSequence`
    (:`then_0`
      (if (== (`.ItemID_4_D9725D3941C812239EFE3E94C6925D23` (break `/Game/UtubeInventory/ItemData/S_ItemSlot` (`local.LocalSourceInventory`))) (`.ItemID_4_D9725D3941C812239EFE3E94C6925D23` (break `/Game/UtubeInventory/ItemData/S_ItemSlot` (`local.LocalDestinationInventory`))))
        (`self.ItemTransfer` (`local.SourceInventory`) (`local.LocalSourceInventory`) (`local.LocalDestinationInventory`) (`local.Index`) (`local.SourceIndex`))
        (else
          (`self.AddtoNewSlot` _itemid _itemquantity (`local.SourceIndex`))
          (`self.AddtoNewSlot` _itemid_2 _itemquantity_2 (`local.Index`)))))
    (:`then_1`
      (`self.UpdateInventory` (`local.SourceInventory`))
      (`self.UpdateInventory`))))